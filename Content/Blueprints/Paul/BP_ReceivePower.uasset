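; BP_ReceivePower is a power receptacle that docks a BP_Battery at BatterySpot and reads its power.
; Trigger overlap casts the same actor to both battery and PlayerCharacter_Paul before releasing the grab, easing the component into place and zeroing its velocity.
; If still colliding a second later, it starts charging and copies Power to RPower, which SetBatteryPower writes back.
; A BPI_Pickup actor leaving the trigger clears both states.
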(event `self.ReceiveBeginPlay`
  (bind _asninja_player_character_bp (cast `/NinjaCharacter/NinjaCharacter/Blueprints/NinjaPlayerCharacter_BP` (`GameplayStatics.GetPlayerCharacter` 0)))
  (set `self.As Ninja Player Character BP` _asninja_player_character_bp))

(event `self.Trigger.OnComponentBeginOverlap`
  (params (OverlappedComponent :type "PrimitiveComponent Object Reference") (OtherActor :type "Actor Object Reference") (OtherComp :type "PrimitiveComponent Object Reference") (OtherBodyIndex :type Integer) (bFromSweep :type Boolean) (SweepResult :type "HitResult Structure (by ref)"))
  (bind _other_comp (`self.Other Comp`))
  (bind _output_get (set `self.Attached Actor` OtherActor))
  (set `self.Other Comp` OtherComp)
  (bind _asbp_battery (cast `/Game/Blueprints/Paul/BP_Battery` OtherActor))
  (set `self.As BP Battery` _asbp_battery)
  (bind _asplayer_character_paul (cast `/Game/Blueprints/Paul/PlayerCharacter_Paul` _output_get))
  (`/Game/Blueprints/Paul/PlayerCharacter_Paul.Stop Grabbing Object` _asplayer_character_paul)
  (`KismetSystemLibrary.MoveComponentTo` (`self.Other Comp`) (`SceneComponent.K2_GetComponentLocation` (`self.Battery Spot`)) (struct) true true 0.1)
  (`PrimitiveComponent.SetPhysicsLinearVelocity` _other_comp (0.0 0.0 0.0) false "None")
  (`PrimitiveComponent.SetPhysicsAngularVelocityInDegrees` _other_comp (0.0 0.0 0.0) false "None")
  (set `self.Is Colliding` true)
  (`KismetSystemLibrary.Delay` 1.0)
  (if (`self.Is Colliding`)
    (set `self.Is Charging` true)
    (set `self.RPower` (`/Game/Blueprints/Paul/BP_Battery.Power` (`self.As BP Battery`)))))

(event `self.Trigger.OnComponentEndOverlap`
  (params (OverlappedComponent :type "PrimitiveComponent Object Reference") (OtherActor :type "Actor Object Reference") (OtherComp :type "PrimitiveComponent Object Reference") (OtherBodyIndex :type Integer))
  (if (`KismetSystemLibrary.DoesImplementInterface` OtherActor "/Game/Blueprints/Paul/BPI_Pickup.BPI_Pickup_C")
    (set `self.Is Colliding` false)
    (`KismetSystemLibrary.PrintString` "DC'd")
    (set `self.Is Charging` false)))

(fn `Set Battery Power`
  (set `/Game/Blueprints/Paul/BP_Battery.Power` (`self.RPower`) (`self.As BP Battery`)))

(fn `UserConstructionScript`)
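; BP_GravityBounds is a spherical gravity zone that sets the gravity of characters inside it using its own location.
; A timer started on BeginPlay calls SetPlayerGravity, which gets every BaseCharacter_BP in the level.
; Characters whose squared distance to the center is within the Bounds sphere's squared scaled radius receive SetGravity with that center.
; Characters outside are left untouched, with no reset on exit.
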(event `self.ReceiveBeginPlay`
  (`KismetSystemLibrary.K2_SetTimerDelegate` (delegate `Update Gravity`)))

(event `Update Gravity`
  (`self.Set Player Gravity`))

(fn `Is Inside Bounds`
  (params (Actor :type "Actor Object Reference"))
  (returns (`Is Inside Bounds` :type Boolean))
  (bind (_returnvalue_x _returnvalue_y _returnvalue_z) (`KismetMathLibrary.BreakVector` (`self.K2_GetActorLocation`)))
  (bind (_returnvalue_x_2 _returnvalue_y_2 _returnvalue_z_2) (`KismetMathLibrary.BreakVector` (`self.K2_GetActorLocation` Actor)))
  (return (< (+ (`KismetMathLibrary.Square` (- _returnvalue_x_2 _returnvalue_x)) (`KismetMathLibrary.Square` (- _returnvalue_y_2 _returnvalue_y)) (`KismetMathLibrary.Square` (- _returnvalue_z_2 _returnvalue_z))) (`KismetMathLibrary.Square` (`SphereComponent.GetScaledSphereRadius` (`self.Bounds`))))))

(fn `Set Player Gravity`
  (bind _outactors (`GameplayStatics.GetAllActorsOfClass` "/Game/Blueprints/Paul/BaseCharacter_BP.BaseCharacter_BP_C"))
  (for _array_element _outactors
    (if (`self.Is Inside Bounds` _array_element)
      (`/Game/Blueprints/Paul/BaseCharacter_BP.SetGravity` _array_element (`self.K2_GetActorLocation`)))))

(fn `UserConstructionScript`)
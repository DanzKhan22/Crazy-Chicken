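; BP_Button is an interactable button that moves power from a BP_GivePower actor to a BP_ReceivePower actor.
; BeginPlay caches the first actor found of each class.
; Interact requires both to be charging, decrements the giver's count once, then loops shifting units until the giver empties or the receiver reaches its cap.
; Each loop step writes both values back, refreshes both battery displays and prints the totals.
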(event `self.ReceiveBeginPlay`
  (bind _outactors (`GameplayStatics.GetAllActorsOfClass` "/Game/Blueprints/Paul/BP_GivePower.BP_GivePower_C"))
  (set `self.Give Power Reference` (`|GetArrayItem` _outactors))
  (bind _outactors_2 (`GameplayStatics.GetAllActorsOfClass` "/Game/Blueprints/Paul/BP_ReceivePower.BP_ReceivePower_C"))
  (set `self.Receive Power Reference` (`|GetArrayItem` _outactors_2)))

(fn `Interact`
  (locals (GPowerRef :type Integer :default 0) (RPowerRef :type Integer :default 0) (`Total Power` :type Integer))
  (bind _receive_power_reference (`self.Receive Power Reference`))
  (bind _give_power_reference (`self.Give Power Reference`))
  (bind _gpowerref (`local.GPowerRef`))
  (if (`/Game/Blueprints/Paul/BP_GivePower.Is Charging` (`self.Give Power Reference`))
    (if (`/Game/Blueprints/Paul/BP_ReceivePower.Is Charging` (`self.Receive Power Reference`))
      (bind _output_get (set `local.GPowerRef` (`/Game/Blueprints/Paul/BP_GivePower.GPower` _give_power_reference)))
      (bind _output_get_2 (set `local.RPowerRef` (`/Game/Blueprints/Paul/BP_ReceivePower.RPower` _receive_power_reference)))
      (if (>= _output_get 0)
        (if (<= _output_get_2 6)
          (`/Engine/EditorBlueprintResources/StandardMacros.DecrementInt` _gpowerref
            (:`  `
              (while (and (> _gpowerref 0) (< (`local.RPowerRef`) 6))
                (bind _result (`/Engine/EditorBlueprintResources/StandardMacros.DecrementInt` (`local.GPowerRef`))
                  (:`  `
                    (bind _result_2 (`/Engine/EditorBlueprintResources/StandardMacros.IncrementInt` (`local.RPowerRef`))
                      (:`  `
                        (bind _output_get_3 (set `/Game/Blueprints/Paul/BP_GivePower.GPower` _result _give_power_reference))
                        (bind _output_get_4 (set `/Game/Blueprints/Paul/BP_ReceivePower.RPower` _result_2 _receive_power_reference))
                        (`/Game/Blueprints/Paul/BP_GivePower.Set Battery Power` (`self.Give Power Reference`))
                        (`/Game/Blueprints/Paul/BP_ReceivePower.Set Battery Power` (`self.Receive Power Reference`))
                        (`KismetSystemLibrary.PrintString` (`KismetStringLibrary.Concat_StrStr` "Giving Ball:" (`KismetStringLibrary.Conv_IntToString` _output_get_3) "Receiving Ball: " (`KismetStringLibrary.Conv_IntToString` _output_get_4)) true true (struct :`G` 0.66 :`B` 1.0 :`A` 1.0) 10.0)))))))))))))

(fn `UserConstructionScript`)
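; A door socket that opens its sliding door when the player inserts a battery with enough power.
; On BeginPlay, the counter lights red segments to match the required power, up to six.
; An overlapping battery is released from the player's grab, snapped into place and stopped, then checked after a short delay.
; Sufficient power flashes the counter green and plays a timeline raising the door; removing the battery only clears the charging flags.
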(event `self.ReceiveBeginPlay`
  (bind _counter (`self.Counter`))
  (bind _asplayer_character_paul (cast `/Game/Blueprints/Paul/PlayerCharacter_Paul` (`GameplayStatics.GetPlayerCharacter` 0)))
  (set `self.As Player Character Paul` _asplayer_character_paul)
  (switch `int` (`self.Power Required`)
    (:`1`
      (`PrimitiveComponent.SetMaterial` _counter 0 "/Game/Materials/RedGlow.RedGlow"))
    (:`2`
      (`PrimitiveComponent.SetMaterial` _counter 0 "/Game/Materials/RedGlow.RedGlow")
      (`PrimitiveComponent.SetMaterial` _counter 1 "/Game/Materials/RedGlow.RedGlow"))
    (:`3`
      (`PrimitiveComponent.SetMaterial` _counter 0 "/Game/Materials/RedGlow.RedGlow")
      (`PrimitiveComponent.SetMaterial` _counter 1 "/Game/Materials/RedGlow.RedGlow")
      (`PrimitiveComponent.SetMaterial` _counter 2 "/Game/Materials/RedGlow.RedGlow"))
    (:`4`
      (`PrimitiveComponent.SetMaterial` _counter 0 "/Game/Materials/RedGlow.RedGlow")
      (`PrimitiveComponent.SetMaterial` _counter 1 "/Game/Materials/RedGlow.RedGlow")
      (`PrimitiveComponent.SetMaterial` _counter 2 "/Game/Materials/RedGlow.RedGlow")
      (`PrimitiveComponent.SetMaterial` _counter 3 "/Game/Materials/RedGlow.RedGlow"))
    (:`5`
      (`PrimitiveComponent.SetMaterial` _counter 0 "/Game/Materials/RedGlow.RedGlow")
      (`PrimitiveComponent.SetMaterial` _counter 1 "/Game/Materials/RedGlow.RedGlow")
      (`PrimitiveComponent.SetMaterial` _counter 2 "/Game/Materials/RedGlow.RedGlow")
      (`PrimitiveComponent.SetMaterial` _counter 3 "/Game/Materials/RedGlow.RedGlow")
      (`PrimitiveComponent.SetMaterial` _counter 4 "/Game/Materials/RedGlow.RedGlow"))
    (:`6`
      (`PrimitiveComponent.SetMaterial` _counter 0 "/Game/Materials/RedGlow.RedGlow")
      (`PrimitiveComponent.SetMaterial` _counter 1 "/Game/Materials/RedGlow.RedGlow")
      (`PrimitiveComponent.SetMaterial` _counter 2 "/Game/Materials/RedGlow.RedGlow")
      (`PrimitiveComponent.SetMaterial` _counter 3 "/Game/Materials/RedGlow.RedGlow")
      (`PrimitiveComponent.SetMaterial` _counter 4 "/Game/Materials/RedGlow.RedGlow")
      (`PrimitiveComponent.SetMaterial` _counter 5 "/Game/Materials/RedGlow.RedGlow"))))

(event `self.Trigger.OnComponentBeginOverlap`
  (params (OverlappedComponent :type "PrimitiveComponent Object Reference") (OtherActor :type "Actor Object Reference") (OtherComp :type "PrimitiveComponent Object Reference") (OtherBodyIndex :type Integer) (bFromSweep :type Boolean) (SweepResult :type "HitResult Structure (by ref)"))
  (bind _other_comp (`self.Other Comp`))
  (bind _counter (`self.Counter`))
  (bind _counter_2 (`self.Counter`))
  (bind _counter_3 (`self.Counter`))
  (set `self.Attached Actor` OtherActor)
  (set `self.Other Comp` OtherComp)
  (bind _asbp_battery (cast `/Game/Blueprints/Paul/BP_Battery` OtherActor))
  (set `self.As BP Battery` _asbp_battery)
  (`/Game/Blueprints/Paul/PlayerCharacter_Paul.Stop Grabbing Object` (`self.As Player Character Paul`))
  (`KismetSystemLibrary.MoveComponentTo` (`self.Other Comp`) (`SceneComponent.K2_GetComponentLocation` (`self.Battery Spot`)) (struct) true true 0.1)
  (`PrimitiveComponent.SetPhysicsLinearVelocity` _other_comp (0.0 0.0 0.0) false "None")
  (`PrimitiveComponent.SetPhysicsAngularVelocityInDegrees` _other_comp (0.0 0.0 0.0) false "None")
  (set `self.Is Colliding` true)
  (`KismetSystemLibrary.Delay` 1.0)
  (if (`self.Is Colliding`)
    (set `self.Is Charging` true)
    (bind _output_get (set `self.Power Received` (`/Game/Blueprints/Paul/BP_Battery.Power` (`self.As BP Battery`))))
    (if (>= _output_get (`self.Power Required`))
      ;[0.06404 1 0] Door Color Change
      (`PrimitiveComponent.SetMaterial` _counter_2 0 "/Game/Materials/GreenGlow.GreenGlow")
      (`PrimitiveComponent.SetMaterial` _counter_2 1 "/Game/Materials/GreenGlow.GreenGlow")
      (`PrimitiveComponent.SetMaterial` _counter_2 2 "/Game/Materials/GreenGlow.GreenGlow")
      (`PrimitiveComponent.SetMaterial` _counter_2 3 "/Game/Materials/GreenGlow.GreenGlow")
      (`PrimitiveComponent.SetMaterial` _counter_2 4 "/Game/Materials/GreenGlow.GreenGlow")
      (`PrimitiveComponent.SetMaterial` _counter_2 5 "/Game/Materials/GreenGlow.GreenGlow")
      (`KismetSystemLibrary.Delay` 0.1)
      (`PrimitiveComponent.SetMaterial` _counter_3 0 "/Game/Materials/BlackGlow.BlackGlow")
      (`PrimitiveComponent.SetMaterial` _counter_3 1 "/Game/Materials/BlackGlow.BlackGlow")
      (`PrimitiveComponent.SetMaterial` _counter_3 2 "/Game/Materials/BlackGlow.BlackGlow")
      (`PrimitiveComponent.SetMaterial` _counter_3 3 "/Game/Materials/BlackGlow.BlackGlow")
      (`PrimitiveComponent.SetMaterial` _counter_3 4 "/Game/Materials/BlackGlow.BlackGlow")
      (`PrimitiveComponent.SetMaterial` _counter_3 5 "/Game/Materials/BlackGlow.BlackGlow")
      (`KismetSystemLibrary.Delay` 0.1)
      (`PrimitiveComponent.SetMaterial` _counter 0 "/Game/Materials/GreenGlow.GreenGlow")
      (`PrimitiveComponent.SetMaterial` _counter 1 "/Game/Materials/GreenGlow.GreenGlow")
      (`PrimitiveComponent.SetMaterial` _counter 2 "/Game/Materials/GreenGlow.GreenGlow")
      (`PrimitiveComponent.SetMaterial` _counter 3 "/Game/Materials/GreenGlow.GreenGlow")
      (`PrimitiveComponent.SetMaterial` _counter 4 "/Game/Materials/GreenGlow.GreenGlow")
      (`PrimitiveComponent.SetMaterial` _counter 5 "/Game/Materials/GreenGlow.GreenGlow")
      (bind (_direction _door_slide) (`Timeline|OpenDoor`)
        (:`Update`
          (`SceneComponent.K2_SetRelativeLocation` (`self.Door`) (`KismetMathLibrary.MakeVector` 0.0 0.0 (`KismetMathLibrary.Lerp` 0.0 600.0 _door_slide)) false false))))))

(event `self.Trigger.OnComponentEndOverlap`
  (params (OverlappedComponent :type "PrimitiveComponent Object Reference") (OtherActor :type "Actor Object Reference") (OtherComp :type "PrimitiveComponent Object Reference") (OtherBodyIndex :type Integer))
  (if (`KismetSystemLibrary.DoesImplementInterface` OtherActor "/Game/Blueprints/Paul/BPI_Pickup.BPI_Pickup_C")
    (set `self.Is Colliding` false)
    (set `self.Is Charging` false)))

(fn `UserConstructionScript`)